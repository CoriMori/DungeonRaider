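; BP_AlterKey is a key-check actor that turns two candle groups' flames blue when the correct key is presented.
; Actors overlapping its Box are passed to the DoorKey component for checking.
; DoorKey's key-correct delegate drives TriggerBlueFlames on both BP_CandleGroup child actors.
; The StartBlue flag invokes the key-correct event at BeginPlay, so the candles can start blue.
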(event OnComponentBeginOverlap(Box)
  (params (OverlappedComponent :type Primitive%20Component%20Object%20Reference) (OtherActor :type Actor%20Object%20Reference) (OtherComp :type Primitive%20Component%20Object%20Reference) (OtherBodyIndex :type Integer) (bFromSweep :type Boolean) (SweepResult :type Hit%20Result%20Structure%20%28by%20ref%29))
  (Class|DoorKey|CheckKey (Variables|Default|GetDoorKey) OtherActor))

(event Custom|OnKeyCorrectDelegate_Event
  (bind _asbp_candle_group (Utilities|Casting|CastToBP_CandleGroup (Variables|/Script/Engine.ChildActorComponent|GetChildActor (Variables|Default|GetBP_CandleGroup))))
  (Default|TriggerBlueFlames _asbp_candle_group)
  (bind _asbp_candle_group_2 (Utilities|Casting|CastToBP_CandleGroup (Variables|/Script/Engine.ChildActorComponent|GetChildActor (Variables|Default|GetBP_CandleGroup1))))
  (Default|TriggerBlueFlames _asbp_candle_group_2))

(event EventBeginPlay
  (EventDispatchers|AssignOnKeyCorrectDelegate (Variables|Default|GetDoorKey) (delegate Custom|OnKeyCorrectDelegate_Event))
  (if (Variables|Default|GetStartBlue)
    (CallFunction|OnKeyCorrectDelegateEvent)))

(fn ConstructionScript)