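; BP_CandleGroup is a candle group prop with three flame components that keeps its flames at zero world rotation, whatever the actor's orientation.
; The Construction Script resets each flame's world rotation, so the correction applies whenever construction runs.
; BeginPlay repeats the same reset once when play starts, with no per-frame update afterward.
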(event EventBeginPlay
  (Transformation|SetWorldRotation (Variables|Default|GetSM-CandleFlame-01) "0, 0, 0" false false)
  (Transformation|SetWorldRotation (Variables|Default|GetSM-CandleFlame-02) "0, 0, 0" false false)
  (Transformation|SetWorldRotation (Variables|Default|GetSM-CandleFlame-03) "0, 0, 0" false false))

(fn ConstructionScript
  (Transformation|SetWorldRotation (Variables|Default|GetSM-CandleFlame-01) "0, 0, 0" false false)
  (Transformation|SetWorldRotation (Variables|Default|GetSM-CandleFlame-02) "0, 0, 0" false false)
  (Transformation|SetWorldRotation (Variables|Default|GetSM-CandleFlame-03) "0, 0, 0" false false))